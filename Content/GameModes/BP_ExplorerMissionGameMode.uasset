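; Explorer mission game mode that sets game-only input at BeginPlay and listens for input-device and mission events.
; It binds an event to the explorer controller's key switch, while SetupInput prints whether keyboard and mouse or controller is active.
; It then binds MissionComplete to the mission game state's completion event.
; Both handlers are placeholders that only print messages.
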(event `self.ReceiveBeginPlay`
  (bind _returnvalue (`GameplayStatics.GetPlayerController` 0))
  (`WidgetBlueprintLibrary.SetInputMode_GameOnly` _returnvalue)
  (bind _asexplorer_controller_bp (cast `/Game/FirstPerson/Blueprints/ExplorerController_BP` _returnvalue))
  (add `/Game/FirstPerson/Blueprints/ExplorerController_BP.KeySwitch` _asexplorer_controller_bp (`|CreateDelegate` :!event `SetupInput`))
  (bind _asmission_game_state (cast `MissionGameState` (`GameplayStatics.GetGameState`)))
  (add `MissionGameState.OnMissionComplete` _asmission_game_state (delegate `MissionComplete`)))

(event `MissionComplete`
  (`KismetSystemLibrary.PrintString` "Mission Complete!"))

(fn `SetupInput`
  (params (NewInputType :type "/Game/Input/E_InputType Enum" :default "NewEnumerator2"))
  (switch `/Game/Input/E_InputType` NewInputType
    (:`NewEnumerator0`
      (`KismetSystemLibrary.PrintString` "Setup Input: Switched to Keyboard and Mouse"))
    (:`NewEnumerator1`
      (`KismetSystemLibrary.PrintString` "Setup Input: Switched to Controller"))))

(fn `UserConstructionScript`)