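; Poison hazard actor that damages first-person characters standing inside its Box volume.
; Box overlap events add and remove characters in a TouchingPlayers list.
; BeginPlay starts a looping one-second timer, apparently meant to drive DamagePlayers, though the bound event is not shown.
; DamagePlayers applies a small fixed damage to each listed character, with debug prints on overlap and damage.
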(event `self.ReceiveBeginPlay`
  (`KismetSystemLibrary.K2_SetTimerDelegate` (`|CreateDelegate` :!event `DamagePlayers`) 1.0 true))

(event `self.Box.OnComponentBeginOverlap`
  (params (OverlappedComponent :type "PrimitiveComponent Object Reference") (OtherActor :type "Actor Object Reference") (OtherComp :type "PrimitiveComponent Object Reference") (OtherBodyIndex :type Integer) (bFromSweep :type Boolean) (SweepResult :type "HitResult Structure (by ref)"))
  (`KismetSystemLibrary.PrintString` (`KismetStringLibrary.Concat_StrStr` (`KismetSystemLibrary.GetDisplayName` OverlappedComponent) " touched by " (`KismetSystemLibrary.GetDisplayName` OtherActor)))
  (bind _asbp_first_person_character (cast `/Game/FirstPerson/Blueprints/BP_FirstPersonCharacter` OtherActor))
  (`KismetArrayLibrary.Array_Add` (`self.TouchingPlayers`) _asbp_first_person_character))

(event `self.Box.OnComponentEndOverlap`
  (params (OverlappedComponent :type "PrimitiveComponent Object Reference") (OtherActor :type "Actor Object Reference") (OtherComp :type "PrimitiveComponent Object Reference") (OtherBodyIndex :type Integer))
  (`KismetSystemLibrary.PrintString` (`KismetStringLibrary.Concat_StrStr` (`KismetSystemLibrary.GetDisplayName` OverlappedComponent) " untouched by " (`KismetSystemLibrary.GetDisplayName` OtherActor)))
  (bind _asbp_first_person_character (cast `/Game/FirstPerson/Blueprints/BP_FirstPersonCharacter` OtherActor))
  (`KismetArrayLibrary.Array_RemoveItem` (`self.TouchingPlayers`) _asbp_first_person_character))

(fn `DamagePlayers`
  (for _array_element (`self.TouchingPlayers`)
    (`GameplayStatics.ApplyDamage` _array_element 1.0 null self)
    (`KismetSystemLibrary.PrintString` (`KismetStringLibrary.Concat_StrStr` "Damaging" (`KismetSystemLibrary.GetDisplayName` _array_element)))))

(fn `UserConstructionScript`)